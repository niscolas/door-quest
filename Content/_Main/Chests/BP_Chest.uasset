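; BP_Chest is an interactable chest that opens once and spawns an item drop.
; While interaction is enabled, focus events use default helpers to toggle outlines on the lid and base and the interaction indicator.
; Interacting plays a timeline that rolls the lid wrapper open, then clears focus, disables interaction and spawns the configured drop class at SpawnPoint, if valid.
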(event `Open`
  (bind _lidwrapper (`self.LidWrapper`))
  (bind (_relativerotation_roll _relativerotation_pitch _relativerotation_yaw) (`KismetMathLibrary.BreakRotator` (`SceneComponent.RelativeRotation` _lidwrapper)))
  (bind (_direction _rotation) (`Timeline|Timeline_Open`)
    (:`Update`
      (`SceneComponent.K2_SetRelativeRotation` _lidwrapper (`KismetMathLibrary.MakeRotator` _rotation _relativerotation_pitch _relativerotation_yaw) false false))
    (:`Finished`
      (`self.LoseInteractionFocus` null)
      (set `self.InteractionEnabled` false)
      (`self.SpawnDrops`))))

(event `self.ReceiveInteractionFocus`
  (params (InteractorActor :type "Actor Object Reference"))
  (if (`self.InteractionEnabled`)
    (`/Game/_Main/Libraries/FunctionLibraries/BPFL_Interactable.Default on Receive Interaction Focus` (`self.OutlineableMeshes`) (`self.ToggleableComponents`))))

(event `self.ReceiveInteraction`
  (params (InteractorActor :type "Actor Object Reference"))
  (if (`self.InteractionEnabled`)
    (`self.Open`)))

(event `self.LoseInteractionFocus`
  (params (InteractorActor :type "Actor Object Reference"))
  (if (`self.InteractionEnabled`)
    (`/Game/_Main/Libraries/FunctionLibraries/BPFL_Interactable.Default on Lost Interaction Focus` (`self.OutlineableMeshes`) (`self.ToggleableComponents`))))

(fn `SpawnDrops`
  (bind (_returnvalue_location _returnvalue_rotation) (`KismetMathLibrary.BreakTransform` (`SceneComponent.K2_GetComponentToWorld` (`self.SpawnPoint`))))
  (if (`KismetSystemLibrary.IsValidClass` (`self.ItemDropBlueprint`))
    (`|SpawnActorFromClass` (`self.ItemDropBlueprint`) (`KismetMathLibrary.MakeTransform` _returnvalue_location _returnvalue_rotation) "AlwaysSpawn" "OverrideRootScale" self null)))

(fn `UserConstructionScript`
  (`KismetArrayLibrary.Array_Add` (`self.OutlineableMeshes`) (`self.Lid`))
  (`KismetArrayLibrary.Array_Add` (`self.OutlineableMeshes`) (`self.Base`))
  (`KismetArrayLibrary.Array_Add` (`self.ToggleableComponents`) (`self.InteractionIndicator`)))