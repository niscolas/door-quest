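; BP_ItemJewel is a pickup jewel item that rotates and bobs in place until a player or other interactor collects it.
; A timeline offsets its Z from the spawn location for floating, while Tick spins it.
; Through the Interactable events it toggles a mesh outline on focus and calls the item component's default pickup on interaction, destroying itself once picked up.
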(event `self.ReceiveBeginPlay`
  (set `self.InitialLocation` (`self.K2_GetActorLocation`))
  (`self.FloatTween`))

(event `self.ReceiveTick`
  (params (DeltaSeconds :type "Float (single-precision)"))
  (`/Game/_Main/Libraries/FunctionLibraries/BPFL_Interactable.Rotate` self))

(event `FloatTween`
  (bind (_direction _locationz) (`Timeline|Timeline_Floating`)
    (:`Update`
      (`self.K2_SetActorLocation` (`KismetMathLibrary.MakeVector` (.x (`self.InitialLocation`)) (.y (`self.InitialLocation`)) (+ (.z (`self.InitialLocation`)) _locationz))))))

(event `self.ReceiveInteractionFocus`
  (params (InteractorActor :type "Actor Object Reference"))
  (`/Game/_Main/Libraries/FunctionLibraries/BPFL_Interactable.EnableOutline` (`self.jewel_jewel`)))

(event `self.LoseInteractionFocus`
  (params (InteractorActor :type "Actor Object Reference"))
  (`/Game/_Main/Libraries/FunctionLibraries/BPFL_Interactable.DisableOutline` (`self.jewel_jewel`)))

(event `self.ReceiveInteraction`
  (params (InteractorActor :type "Actor Object Reference"))
  (`/Game/_Main/Libraries/FunctionLibraries/BPFL_Interactable.DefaultPickup` (`self.DefaultItem`) InteractorActor))

(event `self.DefaultItem.PickedUp`
  (`self.K2_DestroyActor`))

(fn `UserConstructionScript`)