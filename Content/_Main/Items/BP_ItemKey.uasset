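; BP_ItemKey is a key item pickup that rotates and floats in the world until an interactor picks it up.
; A timeline drives the vertical float around its spawn location, while Tick handles rotation.
; Interactable events toggle focus feedback on the mesh and indicator, and route interaction into the DefaultItem component's pickup.
; Shared Default helper functions supply the float, focus and pickup behavior, leaving this Blueprint as thin wiring.
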(event `self.ReceiveBeginPlay`
  (set `self.InitialLocation` (`self.K2_GetActorLocation`))
  (`self.FloatTween`))

(event `self.ReceiveTick`
  (params (DeltaSeconds :type "Float (single-precision)"))
  (`/Game/_Main/Libraries/FunctionLibraries/BPFL_Interactable.Rotate` self))

(event `FloatTween`
  (bind (_direction _locationz) (`Timeline|Timeline_Floating`)
    (:`Update`
      (`/Game/_Main/Libraries/FunctionLibraries/BPFL_Interactable.DefaultFloatUpdate` self (`self.InitialLocation`) _locationz))))

(event `self.ReceiveInteractionFocus`
  (params (InteractorActor :type "Actor Object Reference"))
  (`/Game/_Main/Libraries/FunctionLibraries/BPFL_Interactable.DefaultOnReceiveInteractionFocus` (`self.Mesh`) (`|MakeArray` (`self.InteractionIndicator`))))

(event `self.LoseInteractionFocus`
  (params (InteractorActor :type "Actor Object Reference"))
  (`/Game/_Main/Libraries/FunctionLibraries/BPFL_Interactable.DefaultOnLostInteractionFocus` (`self.Mesh`) (`|MakeArray` (`self.InteractionIndicator`))))

(event `self.ReceiveInteraction`
  (params (InteractorActor :type "Actor Object Reference"))
  (`/Game/_Main/Libraries/FunctionLibraries/BPFL_Interactable.DefaultPickup` (`self.DefaultItem`) InteractorActor))

(event `self.DefaultItem.PickedUp`
  (`/Game/_Main/Libraries/FunctionLibraries/BPFL_Interactable.DefaultOnPickedUp` self))

(fn `UserConstructionScript`)