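; Player character blueprint that handles Enhanced Input movement, look and jump, world interaction and an item inventory.
; DefaultInteractor searches for nearby interactables every tick from the capsule's origin and runs the interact action.
; DefaultInventoryHolder backs the add, decrease and query item wrappers.
; The construction script registers VM_Inventory in the global MVVM collection and binds inventory changes, with a handler that copies slots into that viewmodel.
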(event `self.ReceiveBeginPlay`
  (bind _asplayer_controller (cast `PlayerController` (`self.GetController`)))
  (bind _returnvalue (pcsubsystem `EnhancedInputLocalPlayerSubsystem` _asplayer_controller))
  (`/Engine/EditorBlueprintResources/StandardMacros.IsValid` _returnvalue
    (:`Is Valid`
      (`EnhancedInputSubsystemInterface.AddMappingContext` _returnvalue "/Game/_Main/Input/IMC_Default.IMC_Default" 0 (struct)))))

(event `self.ReceiveTick`
  (params (DeltaSeconds :type "Float (single-precision)"))
  (`DefaultInteractorComponent.FindNearbyInteractables` (`self.DefaultInteractor`)))

(event `EnhancedInput|/Game/_Main/Input/Actions/IA_Jump`
  (params (ActionValue :type Boolean) (ElapsedSeconds :type "Float (double-precision)") (TriggeredSeconds :type "Float (double-precision)") (InputAction :type "InputAction Object Reference" :default "/Game/_Main/Input/Actions/IA_Jump.IA_Jump"))
  (:`Started`
    (`self.Jump`))
  (:`Completed`
    (`self.StopJumping`)))

(event `EnhancedInput|/Game/_Main/Input/Actions/IA_Look`
  (params (ActionValue :type "Vector2D Structure") (ElapsedSeconds :type "Float (double-precision)") (TriggeredSeconds :type "Float (double-precision)") (InputAction :type "InputAction Object Reference" :default "/Game/_Main/Input/Actions/IA_Look.IA_Look"))
  (:`Triggered`
    (`self.Look` ActionValue)))

(event `EnhancedInput|/Game/_Main/Input/Actions/IA_Move`
  (params (ActionValue :type "Vector2D Structure") (ElapsedSeconds :type "Float (double-precision)") (TriggeredSeconds :type "Float (double-precision)") (InputAction :type "InputAction Object Reference" :default "/Game/_Main/Input/Actions/IA_Move.IA_Move"))
  (:`Triggered`
    (`self.Move` ActionValue)))

(event `EnhancedInput|/Game/_Main/Input/Actions/IA_Interact`
  (params (ActionValue :type Boolean) (ElapsedSeconds :type "Float (double-precision)") (TriggeredSeconds :type "Float (double-precision)") (InputAction :type "InputAction Object Reference" :default "/Game/_Main/Input/Actions/IA_Interact.IA_Interact"))
  (:`Triggered`
    (`DefaultInteractorComponent.Interact` (`self.DefaultInteractor`))))

(fn `AddAmountForItemType`
  (params (ItemType :type "ItemTypeDataAsset Object Reference") (Amount :type Integer))
  (returns (ReturnValue :type Boolean))
  (bind _returnvalue (`InventoryHolder.AddAmountForItemType` (`self.DefaultInventoryHolder`) ItemType Amount))
  (return _returnvalue))

(fn `DecreaseAmountForItemType`
  (params (ItemType :type "ItemTypeDataAsset Object Reference") (Amount :type Integer))
  (returns (ReturnValue :type Boolean))
  (bind _returnvalue (`InventoryHolder.DecreaseAmountForItemType` (`self.DefaultInventoryHolder`) ItemType Amount))
  (return _returnvalue))

(fn `InitGlobalInventoryViewmodel`
  (`self.InventoryViewmodel`
    (:`then`
      _)
    (:`else`
      (bind _returnvalue (`|GenericCreateObject` "/Game/_Main/Player/VM_Inventory.VM_Inventory_C"))
      (bind _output_get (set `self.InventoryViewmodel` _returnvalue))))
  (`MVVMViewModelCollectionObject.AddViewModelInstance` (`MVVMGameSubsystem.GetViewModelCollection` (subsystem `MVVMGameSubsystem`)) (make `MVVMViewModelContext` "/Game/_Main/Player/VM_Inventory.VM_Inventory_C" "VM_Inventory") _output_get))

(fn `OnInventoryContentsChanged`
  (set `/Game/_Main/Player/VM_Inventory.Slots` (`DefaultInventoryHolderComponent.GetInventorySlots` (`self.DefaultInventoryHolder`)) (`self.InventoryViewmodel`)))

(fn `TryGetAmountForItemType`
  (params (ItemType :type "ItemTypeDataAsset Object Reference"))
  (returns (Amount :type Integer) (ReturnValue :type Boolean))
  (bind (_amount _returnvalue) (`InventoryHolder.TryGetAmountForItemType` (`self.DefaultInventoryHolder`) ItemType))
  (return _amount _returnvalue))

(fn `UserConstructionScript`
  (set `DefaultInteractorComponent.DetectionOriginComponent` (`self.CapsuleComponent`) (`self.DefaultInteractor`))
  (`self.InitGlobalInventoryViewmodel`)
  (add `DefaultInventoryHolderComponent.InventoryContentsChanged` (`self.DefaultInventoryHolder`) (`|CreateDelegate` :!event `OnInventoryContentsChanged`)))