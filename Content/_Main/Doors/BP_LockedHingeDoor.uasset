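; A hinged door that players can open only after satisfying an item-based lock.
; Interaction asks ItemBasedLockComponent to unlock, then passes to the parent door logic on success or flags a failed attempt on the viewmodel.
; An MVVM viewmodel, built on BeginPlay from the lock's requirements and state, feeds the lock panel widget and tracks lock changes.
; A timeline drives the mesh's yaw to open, and reverses to close.
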(event `self.ReceiveBeginPlay`
  (`self.SetupItemBasedLockPanel`))

(event `self.ItemBasedLockComponent.IsLockedChanged`
  (params (NewValue :type Boolean))
  (set `/Game/_Main/Doors/VM_ItemBasedLock.IsLocked` NewValue (`self.ItemBasedLockViewmodel`)))

(event `self.Open`
  (bind (_direction _rotation) (`Timeline|Timeline` :!label _label)
    (:`Update`
      (`SceneComponent.K2_SetRelativeRotation` (`self.Mesh`) (`KismetMathLibrary.MakeRotator` 0.0 0.0 _rotation) false false))
    (:`Finished`
      (`/Game/_Main/Doors/BPFL_Door.Default on Tween Finished` self))))

(event `self.Close`
  (goto _label :!via `Reverse`))

(event `self.ReceiveInteraction`
  (params (InteractorActor :type "Actor Object Reference"))
  (bind _returnvalue (`ItemBasedLockComponent.TryUnlock` (`self.ItemBasedLockComponent`) InteractorActor))
  (if _returnvalue
    (`parent.ReceiveInteraction` InteractorActor)
    (else
      (`/Game/_Main/Doors/VM_ItemBasedLock.TriggerHasFailedUnlocking` (`self.ItemBasedLockViewmodel`)))))

(fn `SetupItemBasedLockPanel`
  (bind _itembasedlockcomponent (`self.ItemBasedLockComponent`))
  (bind _aswbp_item_based_lock_panel (cast `/Game/_Main/UI/WBP_ItemBasedLockPanel` (`WidgetComponent.GetUserWidgetObject` (`self.ItemBasedLockPanel`))))
  (bind _returnvalue (`|GenericCreateObject` "/Game/_Main/Doors/VM_ItemBasedLock.VM_ItemBasedLock_C" (`ItemBasedLockComponent.GetRequirementsAsInventorySlots` _itembasedlockcomponent) (`ItemBasedLockComponent.IsLocked` _itembasedlockcomponent)))
  (bind _output_get (set `self.ItemBasedLockViewmodel` _returnvalue))
  (set `/Game/_Main/UI/WBP_ItemBasedLockPanel.ItemBasedLockViewmodel` _output_get _aswbp_item_based_lock_panel))

(fn `UserConstructionScript`
  (`KismetArrayLibrary.Array_Add` (`self.OutlinableMeshes`) (`self.Mesh`))
  (`parent.UserConstructionScript`))