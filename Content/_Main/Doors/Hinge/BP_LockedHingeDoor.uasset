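; Hinge door that stays locked until an interacting actor passes its item-based lock component's unlock check.
; A successful unlock runs the inherited interaction, while a failed one triggers failure feedback on the lock panel's viewmodel.
; At BeginPlay it creates a viewmodel from the lock's requirements and state for the panel widget, then syncs lock changes into it.
; Open and close are delegated to a child-actor door visual, whose meshes become outlinable.
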(event `self.ReceiveBeginPlay`
  (`self.SetupItemBasedLockPanel`))

(event `self.ItemBasedLockComponent.IsLockedChanged`
  (params (NewValue :type Boolean))
  (set `/Game/_Main/Doors/VM_ItemBasedLock.IsLocked` NewValue (`self.ItemBasedLockViewmodel`)))

(event `/Game/_Main/Doors/BPI_Door.Open`
  (`/Game/_Main/Doors/Hinge/BP_DefaultHingeDoorVisual.Open` (`self.Visual`)))

(event `/Game/_Main/Doors/BPI_Door.Close`
  (`/Game/_Main/Doors/Hinge/BP_DefaultHingeDoorVisual.Close` (`self.Visual`)))

(event `OnOpenTweenFinished`
  (`/Game/_Main/Doors/BPFL_Door.Default on Open Tween Finished` self))

(event `self.ReceiveInteraction`
  (params (InteractorActor :type "Actor Object Reference"))
  (bind _returnvalue (`ItemBasedLockComponent.TryUnlock` (`self.ItemBasedLockComponent`) InteractorActor))
  (if _returnvalue
    (`parent.ReceiveInteraction` InteractorActor)
    (else
      (`/Game/_Main/Doors/VM_ItemBasedLock.TriggerHasFailedUnlocking` (`self.ItemBasedLockViewmodel`)))))

(fn `SetupItemBasedLockPanel`
  (bind _itembasedlockcomponent (`self.ItemBasedLockComponent`))
  (bind _aswbp_item_based_lock_panel (cast `/Game/_Main/UI/WBP_ItemBasedLockPanel` (`WidgetComponent.GetUserWidgetObject` (`self.ItemBasedLockPanel`))))
  (bind _returnvalue (`|GenericCreateObject` "/Game/_Main/Doors/VM_ItemBasedLock.VM_ItemBasedLock_C" (`ItemBasedLockComponent.GetRequirementsAsInventorySlots` _itembasedlockcomponent) (`ItemBasedLockComponent.IsLocked` _itembasedlockcomponent)))
  (bind _output_get (set `self.ItemBasedLockViewmodel` _returnvalue))
  (set `/Game/_Main/UI/WBP_ItemBasedLockPanel.ItemBasedLockViewmodel` _output_get _aswbp_item_based_lock_panel))

(fn `UserConstructionScript`
  (bind _asbp_default_hinge_door_visual (cast `/Game/_Main/Doors/Hinge/BP_DefaultHingeDoorVisual` (`ChildActorComponent.ChildActor` (`self.BP_SimpleDoorVisual`))))
  (set `self.Visual` _asbp_default_hinge_door_visual)
  (add `/Game/_Main/Doors/Hinge/BP_DefaultHingeDoorVisual.OpenTweenFinished` (`self.Visual`) (`|CreateDelegate` :!event `OnOpenTweenFinished`))
  (`KismetArrayLibrary.Array_Append` (`self.OutlinableMeshes`) (`self.K2_GetComponentsByClass` (`ChildActorComponent.ChildActor` (`self.BP_SimpleDoorVisual`)) "/Script/Engine.StaticMeshComponent"))
  (`parent.UserConstructionScript`))