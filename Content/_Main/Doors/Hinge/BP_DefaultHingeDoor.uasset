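; BP_DefaultHingeDoor is a hinge door that delegates its opening and closing to a child-actor visual, BP_DefaultHingeDoorVisual.
; The construction script caches that visual, binds to its open-tween-finished event and adds its static meshes to OutlinableMeshes before running the parent script.
; Open and Close forward to the visual, while OnOpenTweenFinished hands off to DefaultOnOpenTweenFinished.
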(event `/Game/_Main/Doors/BPI_Door.Open`
  (`/Game/_Main/Doors/Hinge/BP_DefaultHingeDoorVisual.Open` (`self.Visual`)))

(event `/Game/_Main/Doors/BPI_Door.Close`
  (`/Game/_Main/Doors/Hinge/BP_DefaultHingeDoorVisual.Close` (`self.Visual`)))

(event `OnOpenTweenFinished`
  (`/Game/_Main/Doors/BPFL_Door.Default on Open Tween Finished` self))

(fn `UserConstructionScript`
  (bind _asbp_default_hinge_door_visual (cast `/Game/_Main/Doors/Hinge/BP_DefaultHingeDoorVisual` (`ChildActorComponent.ChildActor` (`self.BP_SimpleDoorVisual`))))
  (set `self.Visual` _asbp_default_hinge_door_visual)
  (add `/Game/_Main/Doors/Hinge/BP_DefaultHingeDoorVisual.OpenTweenFinished` (`self.Visual`) (`|CreateDelegate` :!event `OnOpenTweenFinished`))
  (`KismetArrayLibrary.Array_Append` (`self.OutlinableMeshes`) (`self.K2_GetComponentsByClass` (`ChildActorComponent.ChildActor` (`self.BP_SimpleDoorVisual`)) "/Script/Engine.StaticMeshComponent"))
  (`parent.UserConstructionScript`))