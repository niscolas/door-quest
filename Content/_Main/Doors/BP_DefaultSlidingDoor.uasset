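; Default two-panel sliding door Blueprint that opens and closes by animating its left and right meshes.
; On BeginPlay it caches both meshes' relative locations as the base for the motion.
; Open plays a timeline whose updates and completion are delegated to shared default door functions, and Close reverses that timeline.
; The construction script registers both panels as outlinable meshes before running the parent's construction script.
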(event `self.ReceiveBeginPlay`
  (`self.CacheInitialLocation`))

(event `self.Open`
  (bind (_direction _location) (`Timeline|Timeline_Open` :!label _label)
    (:`Update`
      (`/Game/_Main/Doors/BPFL_Door.Default on Sliding Doors Timeline Open Update` _location (`self.LeftMeshInitialLocation`) (`self.RightMeshInitialLocation`) (`self.MeshLeft`) (`self.MeshRight`)))
    (:`Finished`
      (`/Game/_Main/Doors/BPFL_Door.Default on Tween Finished` self))))

(event `self.Close`
  (goto _label :!via `Reverse`))

(fn `CacheInitialLocation`
  (set `self.LeftMeshInitialLocation` (`SceneComponent.RelativeLocation` (`self.MeshLeft`)))
  (set `self.RightMeshInitialLocation` (`SceneComponent.RelativeLocation` (`self.MeshRight`))))

(fn `UserConstructionScript`
  (bind _outlinablemeshes (`self.OutlinableMeshes`))
  (`KismetArrayLibrary.Array_Add` _outlinablemeshes (`self.MeshLeft`))
  (`KismetArrayLibrary.Array_Add` _outlinablemeshes (`self.MeshRight`))
  (`parent.UserConstructionScript`))