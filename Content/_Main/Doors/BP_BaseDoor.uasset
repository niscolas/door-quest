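; BP_BaseDoor is a base door Blueprint that plugs doors into the interaction system and tracks their open and tweening state.
; Focus gain and loss pass outlinable meshes and toggleable components to default handlers for outlining and enabling, and interaction forwards to a default handler.
; The construction script registers the interaction indicator as a toggleable component.
; Setters and getters expose both state flags, with no door movement defined here.
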(event `self.ReceiveInteractionFocus`
  (params (InteractorActor :type "Actor Object Reference"))
  (`/Game/_Main/Libraries/FunctionLibraries/BPFL_Interactable.Default on Receive Interaction Focus` (`self.OutlinableMeshes`) (`self.ToggleableComponents`)))

(event `self.LoseInteractionFocus`
  (params (InteractorActor :type "Actor Object Reference"))
  (`/Game/_Main/Libraries/FunctionLibraries/BPFL_Interactable.Default on Lost Interaction Focus` (`self.OutlinableMeshes`) (`self.ToggleableComponents`)))

(event `self.ReceiveInteraction`
  (params (InteractorActor :type "Actor Object Reference"))
  (`/Game/_Main/Doors/BPFL_Door.Default on Receive Interaction` self))

(event `self.SetIsTweening`
  (params (Value :type Boolean))
  (set `self.IsTweening` Value))

(event `self.SetIsOpen`
  (params (Value :type Boolean))
  (set `self.IsOpen` Value))

(fn `GetIsOpen`
  (returns (Value :type Boolean))
  (return (`self.IsOpen`)))

(fn `GetIsTweening`
  (returns (Value :type Boolean))
  (return (`self.IsTweening`)))

(fn `UserConstructionScript`
  (`KismetArrayLibrary.Array_Add` (`self.ToggleableComponents`) (`self.InteractionIndicator`)))