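; BP_AutomaticSlidingDoor is a sliding door that opens when it receives interaction focus and closes when it loses it.
; The interact event itself is empty, so focus alone drives the door alongside default outline handling.
; A child actor BP_DefaultSlidingDoorVisual performs the movement and reports when its open tween finishes.
; The construction script caches that visual, binds its finish event, adds its static meshes to the outline list and clears toggleable components.
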(event `self.Open`
  (`/Game/_Main/Doors/BPI_Door.Open` (`self.Visual`)))

(event `self.Close`
  (`/Game/_Main/Doors/BPI_Door.Close` (`self.Visual`)))

(event `OnOpenTweenFinished`
  (`/Game/_Main/Doors/BPFL_Door.Default on Open Tween Finished` self))

(event `self.ReceiveInteractionFocus`
  (params (InteractorActor :type "Actor Object Reference"))
  (`/Game/_Main/Libraries/FunctionLibraries/BPFL_Interactable.Default on Receive Interaction Focus` (`self.OutlinableMeshes`) (`self.ToggleableComponents`))
  (`self.Open`))

(event `self.LoseInteractionFocus`
  (params (InteractorActor :type "Actor Object Reference"))
  (`/Game/_Main/Libraries/FunctionLibraries/BPFL_Interactable.Default on Lost Interaction Focus` (`self.OutlinableMeshes`) (`self.ToggleableComponents`))
  (`self.Close`))

(event `self.ReceiveInteraction`
  (params (InteractorActor :type "Actor Object Reference")))

(fn `OnTimelineOpenUpdate`
  (params (Location :type "Float (double-precision)")))

(fn `UserConstructionScript`
  (`parent.UserConstructionScript`)
  (bind _asbp_default_sliding_door_visual (cast `/Game/_Main/Doors/Sliding/BP_DefaultSlidingDoorVisual` (`ChildActorComponent.ChildActor` (`self.BP_DefaultSlidingDoorVisual`))))
  (bind _output_get (set `self.Visual` _asbp_default_sliding_door_visual))
  (add `/Game/_Main/Doors/Sliding/BP_DefaultSlidingDoorVisual.OpenTweenFinished` _output_get (`|CreateDelegate` :!event `OnOpenTweenFinished`))
  (`KismetArrayLibrary.Array_Append` (`self.OutlinableMeshes`) (`self.K2_GetComponentsByClass` (`self.Visual`) "/Script/Engine.StaticMeshComponent"))
  (`KismetArrayLibrary.Array_Clear` (`self.ToggleableComponents`)))