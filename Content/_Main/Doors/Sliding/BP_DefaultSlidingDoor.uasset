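; Default sliding door Blueprint that delegates its opening and closing motion to a separate visual actor held in a child actor component.
; The construction script caches that visual, binds a callback to its open-tween completion and adds its static meshes to the outlinable meshes before running the parent script.
; Open and Close forward to the visual, and the open-tween finished event passes the door to DefaultOnOpenTweenFinished.
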(event `self.Open`
  (`/Game/_Main/Doors/BPI_Door.Open` (`self.Visual`)))

(event `self.Close`
  (`/Game/_Main/Doors/BPI_Door.Close` (`self.Visual`)))

(event `OnOpenTweenFinished`
  (`/Game/_Main/Doors/BPFL_Door.Default on Open Tween Finished` self))

(fn `UserConstructionScript`
  (bind _asbp_default_sliding_door_visual (cast `/Game/_Main/Doors/Sliding/BP_DefaultSlidingDoorVisual` (`ChildActorComponent.ChildActor` (`self.BP_DefaultSlidingDoorVisual`))))
  (bind _output_get (set `self.Visual` _asbp_default_sliding_door_visual))
  (add `/Game/_Main/Doors/Sliding/BP_DefaultSlidingDoorVisual.OpenTweenFinished` _output_get (`|CreateDelegate` :!event `OnOpenTweenFinished`))
  (`KismetArrayLibrary.Array_Append` (`self.OutlinableMeshes`) (`self.K2_GetComponentsByClass` (`ChildActorComponent.ChildActor` (`self.BP_DefaultSlidingDoorVisual`)) "/Script/Engine.StaticMeshComponent"))
  (`parent.UserConstructionScript`))