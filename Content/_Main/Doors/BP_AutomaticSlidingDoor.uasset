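; Automatic double sliding door that opens when it gains interaction focus and closes when it loses it.
; BeginPlay caches both meshes' relative locations, and one timeline, played forward or reversed, drives their slide through shared default functions.
; Focus also toggles outlines on both meshes, which the construction script registers while clearing toggleable components.
; The Interaction event itself does nothing.
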(event `self.ReceiveBeginPlay`
  (`self.CacheInitialLocation`))

(event `self.Open`
  (bind (_direction _location) (`Timeline|Timeline_Open` :!label _label)
    (:`Update`
      (`/Game/_Main/Doors/BPFL_Door.Default on Sliding Doors Timeline Open Update` _location (`self.LeftMeshInitialLocation`) (`self.RightMeshInitialLocation`) (`self.MeshLeft`) (`self.MeshRight`)))
    (:`Finished`
      (`/Game/_Main/Doors/BPFL_Door.Default on Tween Finished` self))))

(event `self.Close`
  (goto _label :!via `Reverse`))

(event `self.ReceiveInteractionFocus`
  (params (InteractorActor :type "Actor Object Reference"))
  (`/Game/_Main/Libraries/FunctionLibraries/BPFL_Interactable.Default On Receive Interaction Focus` (`self.OutlinableMeshes`) (`self.ToggleableComponents`))
  (`self.Open`))

(event `self.LoseInteractionFocus`
  (params (InteractorActor :type "Actor Object Reference"))
  (`/Game/_Main/Libraries/FunctionLibraries/BPFL_Interactable.Default on Lost Interaction Focus` (`self.OutlinableMeshes`) (`self.ToggleableComponents`))
  (`self.Close`))

(event `self.ReceiveInteraction`
  (params (InteractorActor :type "Actor Object Reference")))

(fn `CacheInitialLocation`
  (set `self.LeftMeshInitialLocation` (`SceneComponent.RelativeLocation` (`self.MeshLeft`)))
  (set `self.RightMeshInitialLocation` (`SceneComponent.RelativeLocation` (`self.MeshRight`))))

(fn `OnTimelineOpenUpdate`
  (params (Location :type "Float (double-precision)")))

(fn `UserConstructionScript`
  (bind _outlinablemeshes (`self.OutlinableMeshes`))
  (`parent.UserConstructionScript`)
  (`KismetArrayLibrary.Array_Add` _outlinablemeshes (`self.MeshLeft`))
  (`KismetArrayLibrary.Array_Add` _outlinablemeshes (`self.MeshRight`))
  (`KismetArrayLibrary.Array_Clear` (`self.ToggleableComponents`)))