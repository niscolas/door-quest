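; BP_DefaultHingeDoor is an interactable hinged door that swings open and closed, with default focus handlers applied to its SMCube mesh.
; Interaction calls Open or Close based on IsOpen, playing or reversing one timeline that drives the mesh's relative yaw.
; The timeline's Finished output toggles IsOpen.
; IsTweening gates interaction but clears on every timeline Update, so it does not block input for the whole swing.
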(event `self.ReceiveInteractionFocus`
  (params (InteractorActor :type "Actor Object Reference"))
  (`/Game/_Main/Libraries/FunctionLibraries/BPFL_Interactable.DefaultOnReceiveInteractionFocus` (`self.SM_Cube`)))

(event `self.LoseInteractionFocus`
  (params (InteractorActor :type "Actor Object Reference"))
  (`/Game/_Main/Libraries/FunctionLibraries/BPFL_Interactable.DefaultOnLostInteractionFocus` (`self.SM_Cube`)))

(event `self.ReceiveInteraction`
  (params (InteractorActor :type "Actor Object Reference"))
  (if (`self.IsTweening`)
    _
    (elif (`self.IsOpen`)
      (`self.Close`)
      (else
        (`self.Open`)))))

(event `Open`
  (set `self.IsTweening` true)
  (bind (_direction _rotation) (`Timeline|OpenTimeline` :!label _label)
    (:`Update`
      (`SceneComponent.K2_SetRelativeRotation` (`self.SM_Cube`) (`KismetMathLibrary.MakeRotator` 0.0 0.0 _rotation) false false)
      (set `self.IsTweening` false))
    (:`Finished`
      (if (`self.IsOpen`)
        (set `self.IsOpen` false)
        (else
          (set `self.IsOpen` true))))))

(event `Close`
  (set `self.IsTweening` true)
  (goto _label :!via `Reverse`))

(fn `UserConstructionScript`)